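; BP_HJPet is a companion pet that trails the player and fires bullets.
; Each tick it moves toward the player's PetArrow when over 150 units away, with E toggling following through a parity counter.
; It faces the JHEnemy found at BeginPlay, or copies PetArrow's rotation when none is valid.
; B spawns a bullet at its Arrow; MakeBullet2 spawns a second type, plays a player montage and resets laser timing.
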(event `self.ReceiveBeginPlay`
  (`|ExecutionSequence`
    (:`then_0`
      (bind _asbp_hjplayer (cast `/Game/Blueprints/Han/BP_HJPlayer` (`GameplayStatics.GetPlayerPawn` 0)))
      (set `self.As BP HJPlayer` _asbp_hjplayer))
    (:`then_1`
      ;[1 1 1] Player Controller 받아오기
      (`self.EnableInput` (`GameplayStatics.GetPlayerController` 0)))
    (:`then_2`
      ;[1 1 1] Enemy 위치 구하기 (타겟)
      (bind _returnvalue (`GameplayStatics.GetActorOfClass` "/Script/NierAutomata.JHEnemy"))
      (set `self.JHBossClass` _returnvalue))
    (:`then_3`
      ;[1 1 1] Pet Arrow 변수make
      (bind _asbp_hjplayer_2 (cast `/Game/Blueprints/Han/BP_HJPlayer` (`GameplayStatics.GetPlayerPawn` 0)))
      (set `self.Pet Arrow` (`/Game/Blueprints/Han/BP_HJPlayer.PetArrow` _asbp_hjplayer_2)))))

(event `Key|E`
  (params (Key :type "Key Structure"))
  ;[1 1 1] Pet - 따라오기 해제 (펫 점프할 때)
  (:`Pressed`
    (bind _result (`/Engine/EditorBlueprintResources/StandardMacros.IncrementInt` (`self.PetJump`))
      (:`  `
        (set `self.PetJump` _result)))))

(event `self.ReceiveTick`
  (params (DeltaSeconds :type "Float (single-precision)"))
  (`|ExecutionSequence`
    (:`then_0`
      ;[1 1 1] Pet을 Pet Arrow 컴포넌트로 이동
      (if (> (`KismetMathLibrary.VSize` (- (`self.K2_GetActorLocation`) (`SceneComponent.K2_GetComponentLocation` (`self.Pet Arrow`)))) 150.0)
        (if (== (mod (`self.PetJump`) 2) 0)
          (`self.K2_SetActorLocation` (+ (`self.K2_GetActorLocation`) (* (`GameplayStatics.GetWorldDeltaSeconds`) (`self.speed`) (`KismetMathLibrary.Normal` (- (`SceneComponent.K2_GetComponentLocation` (`self.Pet Arrow`)) (`self.K2_GetActorLocation`)))))))))
    (:`then_1`
      (bind _jhbossclass (`self.JHBossClass`)
        (:`then`
          ;[1 1 1] Pet - Enemy를 향한 방향으로 회전
          (`self.K2_SetActorRotation` (`KismetMathLibrary.FindLookAtRotation` (`self.K2_GetActorLocation`) (`self.K2_GetActorLocation` _jhbossclass))))
        (:`else`
          ;[1 1 1] Pet - No Enemy / Player 방향으로 회전
          (`self.K2_SetActorRotation` (`SceneComponent.K2_GetComponentRotation` (`self.Pet Arrow`))))))))

(event `Key|B`
  (params (Key :type "Key Structure"))
  (:`Pressed`
    (`|SpawnActorFromClass` "/Game/Blueprints/Han/BP_HJBullet.BP_HJBullet_C" (`SceneComponent.K2_GetComponentToWorld` (`self.Arrow`)) "Undefined" "MultiplyWithRoot" null null)))

(fn `MakeBullet2`
  (set `self.bBulletAutoFire` false)
  (`Character.PlayAnimMontage` (`self.As BP HJPlayer`) "/Game/Animation/2B_Montage/MBP_2B_Crouch.MBP_2B_Crouch" 2.0 "None")
  (`|SpawnActorFromClass` "/Game/Blueprints/Han/BP_HJBullet2.BP_HJBullet2_C" (`SceneComponent.K2_GetComponentToWorld` (`self.Arrow`)) "Undefined" "MultiplyWithRoot" null null)
  (set `self.LaserCurrTime` 0.0))

(fn `UserConstructionScript`)