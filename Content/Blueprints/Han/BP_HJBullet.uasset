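; BP_HJBullet is a projectile that homes in on the boss, a JHEnemy actor.
; On BeginPlay it caches the actor returned by GetActorOfClass.
; Each Tick it moves toward that actor's current location at Speed scaled by delta time, or along its own forward vector when the boss is invalid.
; Movement sets the location directly without sweep or rotation, and the graph contains no hit or damage logic.
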(event `self.ReceiveBeginPlay`
  (bind _returnvalue (`GameplayStatics.GetActorOfClass` "/Script/NierAutomata.JHEnemy"))
  (set `self.JHBoss` _returnvalue))

(event `self.ReceiveTick`
  (params (DeltaSeconds :type "Float (single-precision)"))
  (bind _jhboss (`self.JHBoss`)
    (:`then`
      ;[1 1 1] Bullet - Boss 있으면 유도탄
      (`self.K2_SetActorLocation` (+ (`self.K2_GetActorLocation`) (* (`KismetMathLibrary.Normal` (- (`self.K2_GetActorLocation` _jhboss) (`self.K2_GetActorLocation`))) (`self.Speed`) (`GameplayStatics.GetWorldDeltaSeconds`)))))
    (:`else`
      ;[1 1 1] Boss 없으면 앞으로 발사
      (`self.K2_SetActorLocation` (+ (`self.K2_GetActorLocation`) (* (`self.GetActorForwardVector`) (`self.Speed`) (`GameplayStatics.GetWorldDeltaSeconds`)))))))

(fn `UserConstructionScript`)