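; BP_HJBullet is a bullet actor that homes in on a BP_JHEnemy.
; BeginPlay finds a single enemy with GetActorOfClass.
; Each Tick re-aims at that enemy's current location and moves the bullet by Speed scaled by delta time, without sweep or a validity check.
; No hit or overlap logic is implemented.
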(event `self.ReceiveBeginPlay`
  ;[1 1 1] 총알 - Enemy 방향으로 이동
  (bind _returnvalue (`GameplayStatics.GetActorOfClass` "/Game/Blueprints/BP_JHEnemy.BP_JHEnemy_C")))

(event `self.ReceiveTick`
  (params (DeltaSeconds :type "Float (single-precision)"))
  ;[1 1 1] 총알 - Enemy 방향으로 이동
  (`self.K2_SetActorLocation` (+ (`self.K2_GetActorLocation`) (* (`KismetMathLibrary.Normal` (- (`self.K2_GetActorLocation` (stale `self.ReceiveBeginPlay` _returnvalue)) (`self.K2_GetActorLocation`))) (`self.Speed`) (`GameplayStatics.GetWorldDeltaSeconds`)))))

(fn `UserConstructionScript`)