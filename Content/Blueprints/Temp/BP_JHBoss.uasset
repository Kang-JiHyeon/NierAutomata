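; Prototype boss actor with a spinning bottom cylinder and a skeleton enemy state machine.
; Each Tick calls RotateBottom to yaw the cylinder at RotateSpeed scaled by delta time, then switches on EnemyState.
; The Move, Attack, Damage and Die states only print debug strings, an Idle print is unreachable, and the AttackState function is an empty stub.
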(event `self.ReceiveTick`
  (params (DeltaSeconds :type "Float (single-precision)"))
  (`self.RotateBottom` (`self.RotateSpeed`))
  (switch `EEnemyState` (`self.EnemyState`)
    (:`Move`
      (`KismetSystemLibrary.PrintString` "Move"))
    (:`Attack`
      (`KismetSystemLibrary.PrintString` "Atack"))
    (:`Damage`
      (`KismetSystemLibrary.PrintString` "Damage"))
    (:`Die`
      (`KismetSystemLibrary.PrintString` "Die"))))

(fn `AttackState`)

(fn `RotateBottom`
  (params (RotateSpeed :type "Float (double-precision)"))
  (`SceneComponent.K2_AddLocalRotation` (`self.Cylinder_Bottom`) (`KismetMathLibrary.MakeRotator` 0.0 0.0 (* RotateSpeed (`GameplayStatics.GetWorldDeltaSeconds`))) false false))

(fn `UserConstructionScript`)