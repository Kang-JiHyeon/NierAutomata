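; BP_HJWeapon is a weapon actor that follows the player and jumps to the right hand on E.
; On BeginPlay it enables input and caches two arrow components from BP_HJPlayer.
; Tick moves it toward WeaponArrow1 at Speed until within a small stop distance, and always copies that arrow's rotation.
; Pressing E snaps it to WeaponArrow2; release runs one follow step, bypassing the distance check.
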(event `self.ReceiveBeginPlay`
  (`|ExecutionSequence`
    (:`then_0`
      (`self.EnableInput` (`GameplayStatics.GetPlayerController` 0)))
    (:`then_1`
      ;[1 1 1] Player의 Weapon1, Weapon2 Arrow를 가져온다
      (bind _asbp_hjplayer (cast `/Game/Blueprints/BP_HJPlayer` (`GameplayStatics.GetPlayerPawn` 0)))
      (`|ExecutionSequence`
        (:`then_0`
          (set `self.Weapon Arrow 2` (`/Game/Blueprints/BP_HJPlayer.WeaponArrow2` _asbp_hjplayer)))
        (:`then_1`
          (set `self.Weapon Arrow 1` (`/Game/Blueprints/BP_HJPlayer.WeaponArrow1` _asbp_hjplayer)))))))

(event `self.ReceiveTick`
  (params (DeltaSeconds :type "Float (single-precision)"))
  (`|ExecutionSequence`
    (:`then_0`
      ;[1 1 1] 거리차가 50보다 작을 땐 이동 멈춤
      (if (> (`KismetMathLibrary.VSize` (- (`SceneComponent.K2_GetComponentLocation` (`self.Weapon Arrow 1`)) (`self.K2_GetActorLocation`))) 50.0)
        (`self.K2_SetActorLocation` (+ (`self.K2_GetActorLocation`) (* (`GameplayStatics.GetWorldDeltaSeconds`) (`self.Speed`) (`KismetMathLibrary.Normal` (- (`SceneComponent.K2_GetComponentLocation` (`self.Weapon Arrow 1`)) (`self.K2_GetActorLocation`))))) :!label _label)))
    (:`then_1`
      ;[1 1 1] Player 회전에 따라 함께 회전
      (`self.K2_SetActorRotation` (`SceneComponent.K2_GetComponentRotation` (`self.Weapon Arrow 1`))))))

(event `Key|E`
  (params (Key :type "Key Structure"))
  ;[1 1 1] E press -> 오른 손으로 이동
  (:`Pressed`
    (`self.K2_SetActorLocation` (`SceneComponent.K2_GetComponentLocation` (`self.Weapon Arrow 2`))))
  (:`Released`
    (goto _label)))

(fn `UserConstructionScript`)