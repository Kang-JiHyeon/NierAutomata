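; Boss movement component in a test folder that moves its owning actor toward TargetPosition.
; BeginPlay adds the owner's starting height to the target's Z.
; While IsMove is set, Tick steps the owner along a straight line at Speed without sweep, then snaps to the target and stops when close.
; An expanding MoveSpiral is shelved: it is never called, and its angle is multiplied by zero.
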(event `self.ReceiveBeginPlay`
  (bind _output_get (set `self.Owner` (`self.GetOwner`)))
  (bind (_returnvalue_x _returnvalue_y _returnvalue_z) (`KismetMathLibrary.BreakVector` (`Actor.K2_GetActorLocation` _output_get)))
  (set `self.TargetPosition` (+ (`self.TargetPosition`) (`KismetMathLibrary.MakeVector` 0.0 0.0 _returnvalue_z))))

(event `self.ReceiveTick`
  (params (DeltaSeconds :type "Float (single-precision)"))
  (if (`self.bIsMove`)
    (`|ExecutionSequence`
      (:`then_0`
        ;[1 1 1] Target 으로 향하는 방향 구하기
        (set `self.Direction` (- (`self.TargetPosition`) (`Actor.K2_GetActorLocation` (`self.Owner`)))))
      (:`then_1`
        (switch `/Game/Blueprints/Kang/Test/EBossMovementType` (`self.MoveType`)
          (:`NewEnumerator0`
            ;[1 1 1] Straight 이동
            (`Actor.K2_SetActorLocation` (`self.Owner`) (+ (`Actor.K2_GetActorLocation` (`self.Owner`)) (* (`KismetMathLibrary.Normal` (`self.Direction`)) (`self.Speed`) (`GameplayStatics.GetWorldDeltaSeconds`))) false false))))
      (:`then_2`
        ;[1 1 1] Target 위치에 도달했을 때 움직임 멈추기
        (if (< (`KismetMathLibrary.VSize` (`self.Direction`)) 10.0)
          (`Actor.K2_SetActorLocation` (`self.Owner`) (`self.TargetPosition`) false false)
          (set `self.bIsMove` false))))))

(fn `MoveSpiral`
  (bind _returnvalue (+ (`self.SpiralRadius`) (* (`self.CurrTime`) (`self.SpiralExpansionRate`))))
  (bind _owner (`self.Owner`)
    (:`then`
      (bind _output_get (set `self.CurrTime` (+ (`self.CurrTime`) (`GameplayStatics.GetWorldDeltaSeconds`))))
      (bind _returnvalue_2 (* (* _output_get (`self.SpiralSpeed`)) 0.0))
      (bind (_returnvalue_x _returnvalue_y _returnvalue_z) (`KismetMathLibrary.BreakVector` (`Actor.K2_GetActorLocation` _owner)))
      (`Actor.K2_SetActorLocation` _owner (`KismetMathLibrary.MakeVector` (* (`KismetMathLibrary.Cos` _returnvalue_2) _returnvalue) (* _returnvalue (`KismetMathLibrary.Sin` _returnvalue_2)) _returnvalue_z) false false))
    (:`else`)))