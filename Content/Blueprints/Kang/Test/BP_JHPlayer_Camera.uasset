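; BP_JHPlayer_Camera is a test player character with a boss lock-on camera, health and montage attacks.
; On BeginPlay it fills HP, spawns the pet at its arrow, sets game-only input and targets BPCameraLockOn at the JHEnemy boss.
; Debug key W plays the dash montage and E plays Attack1.
; TakeDamage decrements HP and calls the still-empty UpdateHPUI; weapon spawning and skill-overlap logic are disconnected.
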(event EventBeginPlay
  (bind _returnvalue (Game|GetPlayerController 0))
  (Utilities|FlowControl|Sequence
    (:then_0
      ;[1 1 1] 현재 체력 = 최대체력
      (Variables|Default|SetHP (Variables|Default|GetMaxHP)))
    (:then_1
      ;[1 1 1] 시작할 때 Pet을 Arrow에 배치
      (Game|SpawnActorfromClass "/Game/Blueprints/BP_HJPet.BP_HJPet_C" (Transformation|GetWorldTransform (Variables|Default|GetPetArrow)) "Undefined" "MultiplyWithRoot" 0 0))
    (:then_2
      ;[1 1 1] Game start - no mouse cursor
      (Variables|/Script/Engine.PlayerController|SetbShowMouseCursor _returnvalue false)
      (Input|SetInputModeGameOnly _returnvalue false))
    (:then_3
      ;[1 1 1] Boss를 찾아서 Camera Target으로 지정
      (bind _returnvalue_2 (Actor|GetActorOfClass "/Script/NierAutomata.JHEnemy"))
      (bind _output_get (Variables|Default|SetJHEnemy _returnvalue_2))
      (Default|SetCameraandTarget (Variables|Default|GetBP_CameraLockOn) (Variables|Default|GetCamera) _output_get))))

(event EventTick
  (params (DeltaSeconds :type Float%20%28single-precision%29)))

(event Collision|EventActorBeginOverlap
  (params (OtherActor :type Actor%20Object%20Reference)))

(event Input|KeyboardEvents|DebugKeyW
  (params (Key :type Key%20Structure) (ActionValue :type Input%20Action%20Value%20Structure))
  ;[1 1 1] Dash - Animation
  (:Pressed
    (Animation|PlayAnimMontage "/Game/Animation/Montage/MBP_Dash.MBP_Dash" 1.0 "None")))

(event Input|KeyboardEvents|E
  (params (Key :type Key%20Structure))
  ;[1 1 1] Dash - Animation
  ;;[1 1 1] Attack1 - Animation
  (:Pressed
    (Animation|PlayAnimMontage "/Game/Animation/Montage/MBP_Attack1.MBP_Attack1" 1.0 "None")))

(fn ConstructionScript)

(fn UpdateHPUI)

(fn TakeDamage
  (Math|Float|DecrementFloat (Math|Conversions|ToFloat(Integer) (Variables|Default|GetHP))
    (:%20%20
      (CallFunction|UpdateHPUI)
      (return (Variables|Default|GetHP)))))