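; Actor component, apparently a test for bosses, that smoothly turns its owner to face a target.
; It caches the owner on BeginPlay and targets the first player's pawn, with SetTarget able to replace that target.
; While LookAt is true, Tick interpolates the owner's rotation toward the target using RInterpTo.
; Both locations have Z zeroed before the look-at calculation, so the facing stays horizontal.
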(event `self.ReceiveBeginPlay`
  (set `self.Owner` (`self.GetOwner`))
  (`self.SetTarget` (`GameplayStatics.GetPlayerPawn` 0)))

(event `self.ReceiveTick`
  (params (DeltaSeconds :type "Float (single-precision)"))
  (if (`self.bLookAt`)
    (bind _target (`self.Target`)
      (:`then`
        (bind _owner (`self.Owner`)
          (:`then`
            (`Actor.K2_SetActorRotation` (`self.Owner`) (`KismetMathLibrary.RInterpTo` (`Actor.K2_GetActorRotation` (`self.Owner`)) (`KismetMathLibrary.FindLookAtRotation` (* (`Actor.K2_GetActorLocation` _owner) (1.0 1.0 0.0)) (* (`Actor.K2_GetActorLocation` _target) (1.0 1.0 0.0))) (`GameplayStatics.GetWorldDeltaSeconds`) 1.0) false))
          (:`else`)))
      (:`else`))))

(fn `SetTarget`
  (params (NewTarget :type "Actor Object Reference"))
  (set `self.Target` NewTarget))