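; Boss enemy actor that shows its health in a WBP_BossHP screen widget, created at BeginPlay and tracking the enemy on screen.
; The Fsm component's OnChangedHp delegate refreshes the bar from Hp over MaxHp and removes it at zero or below.
; Tick projects the ArrowHPBar location to the viewport and lerps the widget toward it for smoothed movement.
; Game-win pause and widget logic is present but disconnected.
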(event `self.ReceiveBeginPlay`
  (`|ExecutionSequence`
    (:`then_0`
      ;[1 1 1] Boss HP Widget 생성  Viewport 에 추가
      (bind _returnvalue (`|CreateWidget` "/Game/UI/WBP_BossHP.WBP_BossHP_C"))
      (`UserWidget.AddToViewport` _returnvalue 0))
    (:`then_1`
      ;[1 1 1] Boss HP 초기값 설정
      (bind _output_get (set `self.WBP_BossHP` _returnvalue))
      (`/Game/UI/WBP_BossHP.SetPercent` _output_get 1.0))
    (:`then_2`
      ;[1 1 1] OnChangedHp 델리게이트에 UpdateHpBar 함수를 바인드
      (add `JHEnemyFSM.OnChangedHp` (`self.Fsm`) (delegate `OnChangedHp_Event`)))))

(event `OnChangedHp_Event`
  (params (InValue :type Integer))
  ;[1 1 1] OnChangedHp 델리게이트에 UpdateHpBar 함수를 바인드
  (`self.UpdateHPBar` InValue)
  ;[1 1 1] HP<=0 이라면 HP Bar 제거
  (if (<= InValue 0)
    (`Widget.RemoveFromParent` (`self.WBP_BossHP`))))

(event `self.ReceiveTick`
  (params (DeltaSeconds :type "Float (single-precision)"))
  (bind _returnvalue (`KismetMathLibrary.Conv_VectorToVector2D` (`KismetMathLibrary.VLerp` (`KismetMathLibrary.Conv_Vector2DToVector` (`self.WEP_BossHP_Viewport Position`)) (`KismetMathLibrary.Conv_Vector2DToVector` (`SlateBlueprintLibrary.ScreenToViewport` (`PlayerController.ProjectWorldLocationToScreen` (`GameplayStatics.GetPlayerController` 0) (`SceneComponent.K2_GetComponentLocation` (`self.Arrow (HPBar)`)) true))) 0.2)))
  ;[1 1 1] World-> Screen
  (`Widget.SetRenderTranslation` (`self.WBP_BossHP`) _returnvalue)
  (set `self.WEP_BossHP_Viewport Position` _returnvalue))

(event `self.SkeletalMeshComp.OnComponentBeginOverlap`
  (params (OverlappedComponent :type "PrimitiveComponent Object Reference") (OtherActor :type "Actor Object Reference") (OtherComp :type "PrimitiveComponent Object Reference") (OtherBodyIndex :type Integer) (bFromSweep :type Boolean) (SweepResult :type "HitResult Structure (by ref)")))

(fn `UpdateHPBar`
  (params (Value :type Integer))
  (bind _fsm (`self.Fsm`))
  (bind _wbp_bosshp (`self.WBP_BossHP`)
    (:`then`
      (`/Game/UI/WBP_BossHP.SetPercent` _wbp_bosshp (/ (`JHEnemyFSM.Hp` _fsm) (`JHEnemyFSM.MaxHp` _fsm))))
    (:`else`)))

(fn `UserConstructionScript`)