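; BP_Laser is an actor that renders a laser beam with Niagara, ending at the first blocking surface in front of it.
; Each Tick it line traces on the Visibility channel along its forward vector for Distance units.
; The hit location, or the trace end on a miss, drives the beam's LaserEnd parameter.
; The impact effect moves to the hit location and shows only when something is hit.
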(event `self.ReceiveBeginPlay`)

(event `self.ReceiveTick`
  (params (DeltaSeconds :type "Float (single-precision)"))
  (bind _returnvalue (`self.K2_GetActorLocation`))
  (bind _returnvalue_2 (+ _returnvalue (* (`self.GetActorForwardVector`) (`self.Distance`))))
  (set `self.TraceEnd` _returnvalue_2)
  (bind _outhit (`KismetSystemLibrary.LineTraceSingle` _returnvalue _returnvalue_2 "TraceTypeQuery1"))
  (set `self.bHit` (`GameplayStatics.BreakHitResult` _outhit))
  (set `self.HitLocation` (`.Location` (`GameplayStatics.BreakHitResult` _outhit)))
  (`FXSystemComponent.SetVectorParameter` (`self.Niagara_Laser`) "LaserEnd" (select `bool` (`self.bHit`) :`false` (`self.TraceEnd`) :`true` (`self.HitLocation`)))
  (`SceneComponent.SetVisibility` (`self.Niagara_LaserImpact`) (`self.bHit`) false)
  (`SceneComponent.K2_SetWorldLocation` (`self.Niagara_LaserImpact`) (`self.HitLocation`) false false))

(fn `UserConstructionScript`)