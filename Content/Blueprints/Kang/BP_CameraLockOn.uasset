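; Camera lock-on component that turns the first player's view toward a target actor.
; Setter functions supply the camera and target; while the target is valid, Tick interpolates control rotation toward the look-at rotation from camera to target.
; A forward sphere trace for picking a hit actor and toggling lock state is present but disconnected, so targets come only through the setters.
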(event `self.ReceiveTick`
  (params (DeltaSeconds :type "Float (single-precision)"))
  (bind _returnvalue (`Pawn.GetController` (`GameplayStatics.GetPlayerPawn` 0)))
  ;[1 1 1] Set Target Lock Rotation
  (`self.LockOnTarget`
    (:`then`
      (`Controller.SetControlRotation` _returnvalue (`KismetMathLibrary.RInterpTo` (`Actor.K2_GetActorRotation` _returnvalue) (`KismetMathLibrary.FindLookAtRotation` (`SceneComponent.K2_GetComponentLocation` (`self.Camera`)) (`Actor.K2_GetActorLocation` (`self.LockOnTarget`))) (`GameplayStatics.GetWorldDeltaSeconds`) (`self.RotationInterpSpeed`))))
    (:`else`)))

(event `Key|Tab`
  (params (Key :type "Key Structure"))
  ;[1 1 1] Target Look Trace And Hit
)

(fn `SetCamera`
  (params (TargetCamera :type "CameraComponent Object Reference"))
  (set `self.Camera` TargetCamera))

(fn `SetCameraAndTarget`
  (params (NewCamera :type "CameraComponent Object Reference") (NewTarget :type "Actor Object Reference"))
  (set `self.Camera` NewCamera)
  (set `self.LockOnTarget` NewTarget))

(fn `SetLockOnTarget`
  (params (NewTarget :type "Actor Object Reference"))
  (set `self.LockOnTarget` NewTarget))