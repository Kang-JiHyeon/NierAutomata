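; Boss health bar actor that hosts a WBP_BossHP widget and floats it toward the player's view.
; Each Tick it looks up BP_HJPlayer, moves toward its CameraArrow until within 50 units, and copies the arrow's rotation.
; TakeBDamage decrements the internal Hp and refreshes the widget's HP ratio.
; UpdateHpUI sets that ratio from a supplied value without changing Hp, and prints it.
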(event `self.ReceiveBeginPlay`
  ;[1 1 1] Camera Arrow의 위치를 파악 후, Camera Arrow 위치를 향하도록 한다
  (`|ExecutionSequence`
    (:`then_0`
      (set `self.Hp` (`self.MaxHp`)))
    (:`then_1`
      (bind _aswbp_boss_hp (cast `/Game/UI/WBP_BossHP` (`WidgetComponent.GetWidget` (`self.Widget`))))
      (set `self.WBP_BossHP` _aswbp_boss_hp)
      (`self.UpdateBossBHP`))
    (:`then_2`
      (bind _returnvalue (`GameplayStatics.GetActorOfClass` "/Game/Blueprints/Han/BP_HJPlayer.BP_HJPlayer_C" :!label _label))
      (set `self.Dir` (`KismetMathLibrary.Normal` (- (`SceneComponent.K2_GetComponentLocation` (`/Game/Blueprints/Han/BP_HJPlayer.CameraArrow` _returnvalue)) (`self.K2_GetActorLocation`)))))))

(event `self.ReceiveTick`
  (params (DeltaSeconds :type "Float (single-precision)"))
  ;[1 1 1] Boss HP Widget을 Camera Arrow 이동한다
  (`|ExecutionSequence`
    (:`then_0`
      (goto _label))
    (:`then_1`
      (if (> (`KismetMathLibrary.VSize` (- (`SceneComponent.K2_GetComponentLocation` (`/Game/Blueprints/Han/BP_HJPlayer.CameraArrow` (stale `self.ReceiveBeginPlay` _returnvalue))) (`self.K2_GetActorLocation`))) 50.0)
        (`self.K2_SetActorLocation` (+ (`self.K2_GetActorLocation`) (* DeltaSeconds (`self.Dir`) (`self.Speed`))))))
    (:`then_2`
      ;[1 1 1] CameraArrow 방향과 위젯 회전 방향을 동일하게 한다
      (bind _returnvalue (`GameplayStatics.GetActorOfClass` "/Game/Blueprints/Han/BP_HJPlayer.BP_HJPlayer_C")))
    (:`then_3`
      (`self.K2_SetActorRotation` (`SceneComponent.K2_GetComponentRotation` (`/Game/Blueprints/Han/BP_HJPlayer.CameraArrow` _returnvalue))))))

(fn `TakeBDamage`
  (returns (BHp :type Integer))
  (`/Engine/EditorBlueprintResources/StandardMacros.DecrementInt` (`self.Hp`)
    (:`  `
      (`self.UpdateBossBHP`)
      (return (`self.Hp`)))))

(fn `UpdateBossBHP`
  (set `/Game/UI/WBP_BossHP.HP` (/ (`KismetMathLibrary.Conv_IntToDouble` (`self.Hp`)) (`self.MaxHp`)) (`self.WBP_BossHP`)))

(fn `UpdateHpUI`
  (params (NewHP :type Integer))
  (bind _maxhp (`self.MaxHp`))
  (if (> _maxhp 0)
    (bind _output_get (set `/Game/UI/WBP_BossHP.HP` (/ (`KismetMathLibrary.Conv_IntToDouble` NewHP) _maxhp) (`self.WBP_BossHP`)))
    (`KismetSystemLibrary.PrintString` (`KismetStringLibrary.Conv_DoubleToString` _output_get))))

(fn `UserConstructionScript`)