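; BP_HJPlayer is the player character, with HP, a companion pet and a weapon.
; BeginPlay fills HP to max, spawns BP_HJPet and BP_HJWeapon at arrow component transforms, and sets game-only input with a hidden cursor.
; E plays the horizontal attack montage and a debug W key plays the dash montage.
; TakeDamage decrements HP, calls UpdateHPUI, which is still an empty stub, and returns HP.
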(event EventBeginPlay
  (bind _returnvalue (Game|GetPlayerController 0))
  (Utilities|FlowControl|Sequence
    (:then_0
      ;[1 1 1] 현재 체력 = 최대체력
      (Variables|Default|SetHP (Variables|Default|GetMaxHP)))
    (:then_1
      ;[1 1 1] 시작할 때 Pet을 Arrow에 배치
      (Game|SpawnActorfromClass "/Game/Blueprints/BP_HJPet.BP_HJPet_C" (Transformation|GetWorldTransform (Variables|Default|GetPetArrow)) "Undefined" "MultiplyWithRoot" 0 0))
    (:then_2
      ;[1 1 1] Game start - no mouse cursor
      (Variables|/Script/Engine.PlayerController|SetbShowMouseCursor _returnvalue false)
      (Input|SetInputModeGameOnly _returnvalue false))
    (:then_3
      ;[1 1 1] 시작할 때 Weapon - back position
      (Game|SpawnActorfromClass "/Game/Blueprints/BP_HJWeapon.BP_HJWeapon_C" (Transformation|GetWorldTransform (Variables|Default|GetWeaponArrow1)) "Undefined" "MultiplyWithRoot" 0 0))))

(event Collision|EventActorBeginOverlap
  (params (OtherActor :type Actor%20Object%20Reference)))

(event EventTick
  (params (DeltaSeconds :type Float%20%28single-precision%29)))

(event Input|KeyboardEvents|DebugKeyW
  (params (Key :type Key%20Structure :default "None") (ActionValue :type Input%20Action%20Value%20Structure))
  (:Pressed
    (Animation|PlayAnimMontage "/Game/Animation/MBP_Dash.MBP_Dash" 1.0 "None")))

(event Input|KeyboardEvents|E
  (params (Key :type Key%20Structure :default "None"))
  (:Pressed
    (Animation|PlayAnimMontage "/Game/Animation/MBP_AttackHorizontal.MBP_AttackHorizontal" 1.0 "None")))

(event Input|KeyboardEvents|R
  (params (Key :type Key%20Structure :default "None")))

(fn ConstructionScript)

(fn UpdateHPUI)

(fn TakeDamage
  (Math|Float|DecrementFloat (Math|Conversions|ToFloat(Integer) (Variables|Default|GetHP))
    (:%20%20
      (CallFunction|UpdateHPUI)
      (return (Variables|Default|GetHP)))))