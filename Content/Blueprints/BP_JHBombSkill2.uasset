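; BP_JHBombSkill2 is a bomb skill actor that fires timed volleys of BP_JHBomb2 from ten fire-position components.
; While Attack is true, Tick accumulates time and, every FireTime, spawns a bomb at each position, calls Fire with the current force and prints that force.
; After each volley, SetForceIndex cycles through the Forces array and UpdateAttack clears Attack once the volley count reaches FireCount.
; Nothing in this graph sets Attack to true or resets the volley count.
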(event `self.ReceiveBeginPlay`
  (set `self.FirePositions` (`|MakeArray` (`self.FirePos1`) (`self.FirePos2`) (`self.FirePos3`) (`self.FirePos4`) (`self.FirePos5`) (`self.FirePos6`) (`self.FirePos7`) (`self.FirePos8`) (`self.FirePos9`) (`self.FirePos10`))))

(event `self.ReceiveTick`
  (params (DeltaSeconds :type "Float (single-precision)"))
  (bind _output (`|GetArrayItem` (`self.Forces`) (`self.CurrForceIndex`)))
  (if (`self.bAttack`)
    ;[1 1 1] FireTime만큼 지날 때마다 Bomb 생성
    (bind _output_get (set `self.CurrTime` (+ (`self.CurrTime`) (`GameplayStatics.GetWorldDeltaSeconds`))))
    (if (>= _output_get (`self.FireTime`))
      (set `self.CurrTime` 0.0)
      ;[1 1 1] Bomb 생성
      (for _array_element (`self.FirePositions`)
        (bind _returnvalue (`|SpawnActorFromClass` "/Game/Blueprints/BP_JHBomb2.BP_JHBomb2_C" (`KismetMathLibrary.MakeTransform` (`SceneComponent.K2_GetComponentLocation` _array_element) (`SceneComponent.K2_GetComponentRotation` _array_element)) "Undefined" "MultiplyWithRoot" null null))
        ;[1 1 1] Bomb의 Force 설정
        (`/Game/Blueprints/BP_JHBomb2.Fire` _returnvalue _output)
        (`KismetSystemLibrary.PrintString` (`KismetStringLibrary.Conv_DoubleToString` _output)))
      ;[1 1 1] 제어 값 업데이트
      (`self.SetForceIndex`)
      (`self.UpdateAttack`))))

(fn `SetForceIndex`
  (set `self.CurrForceIndex` (mod (+ (`self.CurrForceIndex`) 1) (`KismetArrayLibrary.Array_Length` (`self.Forces`)))))

(fn `UpdateAttack`
  (bind _output_get (set `self.CurrFireCount` (+ (`self.CurrFireCount`) 1)))
  (if (>= _output_get (`self.FireCount`))
    (set `self.bAttack` false)))

(fn `UserConstructionScript`)