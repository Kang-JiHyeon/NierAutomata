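; Rotating laser actor that fires colored particle beams from four arrow components.
; BeginPlay collects the arrows and spawns a beam emitter for each, using the particle system matching the selected color.
; Every Tick, a visibility line trace per arrow clips its beam at the first hit or full length and moves the emitter to follow.
; When rotation is enabled, Tick also increments a separate Arrow component's yaw by the speed value, without delta-time scaling.
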(event `self.ReceiveBeginPlay`
  ;[1 1 1] Add all the arrows to the arrows array
  (bind _returnvalue (`KismetArrayLibrary.Array_Add` (`self.Arrows`) (`self.Arrow1`)))
  (`KismetArrayLibrary.Array_Insert` (`self.Emietters`) (`self.Emietter`) _returnvalue)
  (bind _returnvalue_2 (`KismetArrayLibrary.Array_Add` (`self.Arrows`) (`self.Arrow2`)))
  (`KismetArrayLibrary.Array_Insert` (`self.Emietters`) (`self.Emietter_0`) _returnvalue_2)
  (bind _returnvalue_3 (`KismetArrayLibrary.Array_Add` (`self.Arrows`) (`self.Arrow3`)))
  (`KismetArrayLibrary.Array_Insert` (`self.Emietters`) (`self.Emietter_1`) _returnvalue_3)
  (bind _returnvalue_4 (`KismetArrayLibrary.Array_Add` (`self.Arrows`) (`self.Arrow4`)))
  (`KismetArrayLibrary.Array_Insert` (`self.Emietters`) (`self.Emietter_2`) _returnvalue_4)
  ;[1 1 1] Create a beam out of all the arrows
  (`self.Beam`))

(event `self.ReceiveTick`
  (params (DeltaSeconds :type "Float (single-precision)"))
  (bind _arrow (`self.Arrow`))
  (bind (_returnvalue_roll _returnvalue_pitch _returnvalue_yaw) (`KismetMathLibrary.BreakRotator` (`SceneComponent.K2_GetComponentRotation` _arrow)))
  ;[1 1 1] Each tick
  (`|ExecutionSequence`
    (:`then_0`
      ;[1 1 1] Loop all arrows
      (for (_array_element _array_index) (`self.Arrows`)
        (bind _returnvalue (`SceneComponent.K2_GetComponentLocation` _array_element))
        (bind _returnvalue_2 (+ _returnvalue (* (`KismetMathLibrary.Conv_RotatorToVector` (`SceneComponent.K2_GetComponentRotation` _array_element)) (`KismetSystemLibrary.MakeLiteralDouble` (`self.Beam lenght`)))))
        (set `self.Beam end point` _returnvalue_2)
        ;[1 1 1] Detect if there is any object blocking the way
        (bind (_outhit _returnvalue_3) (`KismetSystemLibrary.LineTraceSingle` _returnvalue _returnvalue_2 "TraceTypeQuery1" true))
        (if _returnvalue_3
          ;[1 1 1] If hit, set the end point to the hit location
          (bind _output_get (set `self.Beam end point` (`.ImpactPoint` (`GameplayStatics.BreakHitResult` _outhit)))))
        (bind _output (`|GetArrayItem` (`self.Emietters`) _array_index))
        ;[1 1 1] Replace the end and start points of the beam
        (`ParticleSystemComponent.SetBeamEndPoint` _output 0 _output_get)
        (`SceneComponent.K2_SetWorldLocation` _output _returnvalue false false)))
    (:`then_1`
      ;[1 1 1] Each tick, if the rotation is enabled, rotate the arrows according to the rotation speed
      (if (`self.Rotation`)
        (`SceneComponent.K2_SetWorldRotation` _arrow (`KismetMathLibrary.MakeRotator` _returnvalue_roll _returnvalue_pitch (+ _returnvalue_yaw (`self.Speed`))) false false)))))

(fn `Beam`
  (for (_array_element _array_index) (`self.Arrows`)
    (bind _returnvalue (`SceneComponent.K2_GetComponentLocation` _array_element))
    (bind _returnvalue_2 (+ _returnvalue (* (`KismetMathLibrary.Conv_RotatorToVector` (`SceneComponent.K2_GetComponentRotation` _array_element)) (`KismetSystemLibrary.MakeLiteralDouble` (`self.Beam lenght`)))))
    (set `self.Beam end point` _returnvalue_2)
    ;[1 1 1] Check if there is an object blocking the way
    (bind (_outhit _returnvalue_3) (`KismetSystemLibrary.LineTraceSingle` _returnvalue _returnvalue_2 "TraceTypeQuery1" true))
    (if _returnvalue_3
      ;[1 1 1] If hit, set the end point to the hit location
      (bind _output_get (set `self.Beam end point` (`.ImpactPoint` (`GameplayStatics.BreakHitResult` _outhit)))))
    ;[1 1 1] Use this function to create the beam according to the start and the end point
    (`self.Create beam` (`SceneComponent.K2_GetComponentLocation` _array_element) _output_get _array_index)))

(fn `Create beam`
  (params (Start :type "Vector Structure") (End :type "Vector Structure") (Index :type Integer))
  ;[1 1 1] Use this function to get the particle system corresponding to the selected color
  (bind _out (`self.Get Color` (`self.Color`)))
  ;[1 1 1] Create the particle and add it to the list of existing particles
  (bind _returnvalue (`GameplayStatics.SpawnEmitterAtLocation` _out Start))
  (`KismetArrayLibrary.Array_Set` (`self.Emietters`) Index _returnvalue)
  (`ParticleSystemComponent.SetBeamEndPoint` _returnvalue 0 End))

(fn `Get Color`
  (params (Color :type "/Game/Laser/Blueprints/Others/Colors Enum" :default "NewEnumerator0"))
  (returns (Out :type "ParticleSystem Object Reference"))
  ;[1 1 1] Depending on the selected color, output the corresponding laser particle system
  (switch `/Game/Laser/Blueprints/Others/Colors` Color
    (:`NewEnumerator0`
      (return "/Game/Laser/Particles/Laser_Blue.Laser_Blue"))
    (:`NewEnumerator1`
      (return "/Game/Laser/Particles/Laser_LightBlue.Laser_LightBlue"))
    (:`NewEnumerator2`
      (return "/Game/Laser/Particles/Laser_Purple.Laser_Purple"))
    (:`NewEnumerator3`
      (return "/Game/Laser/Particles/Laser_Red.Laser_Red"))
    (:`NewEnumerator4`
      (return "/Game/Laser/Particles/Laser_Pink.Laser_Pink"))
    (:`NewEnumerator5`
      (return "/Game/Laser/Particles/Laser_Orange.Laser_Orange"))
    (:`NewEnumerator6`
      (return "/Game/Laser/Particles/Laser_Yellow.Laser_Yellow"))
    (:`NewEnumerator7`
      (return "/Game/Laser/Particles/Laser_Green.Laser_Green"))
    (:`NewEnumerator8`
      (return "/Game/Laser/Particles/Laser_White.Laser_White"))
    (:`NewEnumerator9`
      (return "/Game/Laser/Particles/Laser_Off.Laser_Off"))))

(fn `UserConstructionScript`)