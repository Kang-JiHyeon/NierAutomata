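; Configurable laser actor that sweeps a colored particle beam between spline points, back and forth along the spline.
; BeginPlay spawns the emitter for the selected color, then loops on a delay derived from Speed to step the target point, reversing at either end.
; Tick eases the Arrow toward the target using Speed, then line-traces along it so the beam stops at blockers or its maximum length.
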(event `self.ReceiveTick`
  (params (DeltaSeconds :type "Float (single-precision)"))
  (bind _arrow (`self.Arrow`))
  (bind _arrow_2 (`self.Arrow`))
  (bind _emietter (`self.Emietter`))
  (bind _returnvalue (`SceneComponent.K2_GetComponentLocation` _arrow_2))
  (bind _returnvalue_2 (`SceneComponent.K2_GetComponentLocation` _arrow))
  (bind _returnvalue_3 (+ _returnvalue (* (`KismetMathLibrary.Conv_RotatorToVector` (`SceneComponent.K2_GetComponentRotation` _arrow_2)) (`KismetSystemLibrary.MakeLiteralDouble` (`self.Beam lenght`)))))
  ;[1 1 1] Move the beam to the targeted spline point
  (`SceneComponent.K2_SetWorldRotation` (`self.Arrow`) (`KismetMathLibrary.RInterpTo` (`SceneComponent.K2_GetComponentRotation` _arrow) (`KismetMathLibrary.FindLookAtRotation` _returnvalue_2 (`self.BeamTarget`)) DeltaSeconds (`self.Speed`)) false false)
  ;[1 1 1] Create the beam
  ;;[1 1 1] Check if there is an object blocking the way
  (bind (_outhit _returnvalue_4) (`KismetSystemLibrary.LineTraceSingle` _returnvalue _returnvalue_3 "TraceTypeQuery1" true))
  (if _returnvalue_4
    (set `self.Beam end point` (`.ImpactPoint` (`GameplayStatics.BreakHitResult` _outhit)))
    (else
      (set `self.Beam end point` _returnvalue_3)))
  (`ParticleSystemComponent.SetBeamEndPoint` _emietter 0 (`self.Beam end point`))
  (`SceneComponent.K2_SetWorldLocation` _emietter _returnvalue_2 false false))

(event `self.ReceiveBeginPlay`
  (bind _point (`self.Point`))
  (bind _point_2 (`self.Point`))
  ;[1 1 1] Create the beam at the start of the game
  (`self.SpawnBeam`)
  ;[1 1 1] Set the target of the laser to the location of the spline point
  (set `self.BeamTarget` (`SplineComponent.GetLocationAtSplinePoint` (`self.Spline`) (`self.Point`) "World") :!label _label)
  ;[1 1 1] Add 1 or remove 1 to the variable that contains the id of the next spline point
  (if (`self.Inc?`)
    (if (== (`self.Point`) (- (`SplineComponent.GetNumberOfSplinePoints` (`self.Spline`)) 1))
      (set `self.Inc?` false)
      (bind _result (`/Engine/EditorBlueprintResources/StandardMacros.DecrementInt` _point_2)
        (:`  `
          (set `self.Point` _result)))
      (else
        (bind _result_2 (`/Engine/EditorBlueprintResources/StandardMacros.IncrementInt` _point_2)
          (:`  `
            (set `self.Point` _result_2)))))
    (elif (== (`self.Point`) 0)
      (bind _result_3 (`/Engine/EditorBlueprintResources/StandardMacros.IncrementInt` _point)
        (:`  `
          (set `self.Point` _result_3)
          (set `self.Inc?` true)))
      (else
        (bind _result_4 (`/Engine/EditorBlueprintResources/StandardMacros.DecrementInt` _point)
          (:`  `
            (set `self.Point` _result_4))))))
  ;[1 1 1] Loop the process by adding the user specified time
  (`KismetSystemLibrary.Delay` (+ (`self.Speed`) 0.1))
  (goto _label))

(fn `Create beam`
  (params (Start :type "Vector Structure") (End :type "Vector Structure"))
  ;[1 1 1] Use this function to get the particle system corresponding to the selected color
  (bind _out (`self.Get Color` (`self.Color`)))
  ;[1 1 1] Create the laser
  (bind _returnvalue (`GameplayStatics.SpawnEmitterAtLocation` _out Start))
  ;[1 1 1] Set the end point
  (bind _output_get (set `self.Emietter` _returnvalue))
  (`ParticleSystemComponent.SetBeamEndPoint` _output_get 0 End))

(fn `Get Color`
  (params (Color :type "/Game/Laser/Blueprints/Others/Colors Enum" :default "NewEnumerator0"))
  (returns (Out :type "ParticleSystem Object Reference"))
  ;[1 1 1] Depending on the selected color, output the corresponding laser particle system
  (switch `/Game/Laser/Blueprints/Others/Colors` Color
    (:`NewEnumerator0`
      (return "/Game/Laser/Particles/Laser_Blue.Laser_Blue"))
    (:`NewEnumerator1`
      (return "/Game/Laser/Particles/Laser_LightBlue.Laser_LightBlue"))
    (:`NewEnumerator2`
      (return "/Game/Laser/Particles/Laser_Purple.Laser_Purple"))
    (:`NewEnumerator3`
      (return "/Game/Laser/Particles/Laser_Red.Laser_Red"))
    (:`NewEnumerator4`
      (return "/Game/Laser/Particles/Laser_Pink.Laser_Pink"))
    (:`NewEnumerator5`
      (return "/Game/Laser/Particles/Laser_Orange.Laser_Orange"))
    (:`NewEnumerator6`
      (return "/Game/Laser/Particles/Laser_Yellow.Laser_Yellow"))
    (:`NewEnumerator7`
      (return "/Game/Laser/Particles/Laser_Green.Laser_Green"))
    (:`NewEnumerator8`
      (return "/Game/Laser/Particles/Laser_White.Laser_White"))
    (:`NewEnumerator9`
      (return "/Game/Laser/Particles/Laser_Off.Laser_Off"))))

(fn `SpawnBeam`
  (bind _arrow (`self.Arrow`))
  (bind _returnvalue (`SceneComponent.K2_GetComponentLocation` _arrow))
  (bind _returnvalue_2 (+ _returnvalue (* (`KismetMathLibrary.Conv_RotatorToVector` (`SceneComponent.K2_GetComponentRotation` _arrow)) (`KismetSystemLibrary.MakeLiteralDouble` (`self.Beam lenght`)))))
  (set `self.Beam end point` _returnvalue_2)
  ;[1 1 1] Detect if there is any object blocking the way
  (bind (_outhit _returnvalue_3) (`KismetSystemLibrary.LineTraceSingle` _returnvalue _returnvalue_2 "TraceTypeQuery1" true))
  (if _returnvalue_3
    (bind _output_get (set `self.Beam end point` (`.ImpactPoint` (`GameplayStatics.BreakHitResult` _outhit)))))
  ;[1 1 1] Use this function to create the beam according to the defined start and end point
  (`self.Create beam` (`SceneComponent.K2_GetComponentLocation` (`self.Arrow`)) _output_get))

(fn `UserConstructionScript`)